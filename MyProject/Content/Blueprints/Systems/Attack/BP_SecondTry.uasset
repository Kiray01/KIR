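; BP_SecondTry is an attack projectile actor that deals damage on overlap and destroys itself after a short fixed lifetime.
; Its sphere overlap ignores BP_CharacterBase actors and applies BaseHit damage to other actors implementing the BPI_Combat interface.
; After a hit, ProjectileEffect selects the result: Regular destroys the projectile, while Explode calls an empty placeholder event.
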(event OnComponentBeginOverlap(Sphere1)
  (params (OverlappedComponent :type Primitive%20Component%20Object%20Reference) (OtherActor :type Actor%20Object%20Reference) (OtherComp :type Primitive%20Component%20Object%20Reference) (OtherBodyIndex :type Integer) (bFromSweep :type Boolean) (SweepResult :type Hit%20Result%20Structure%20%28by%20ref%29))
  (Utilities|Casting|CastToBP_CharacterBase OtherActor
    (:CastFailed
      (bind _asbpi_combat (Utilities|Casting|CastToBPI_Combat OtherActor))
      (Default|TakeDamage _asbpi_combat (Variables|Default|GetBaseHit))
      (switch Utilities|FlowControl|Switch|SwitchonMagicMissile_Effecte (Variables|Default|GetProjectileEffect)
        (:NewEnumerator0
          (Actor|DestroyActor))
        (:NewEnumerator2
          ;[1 1 1] place holder
          (CallFunction|Exlode))))))

(event Custom|exlode)

(event EventBeginPlay
  (Utilities|FlowControl|Delay 5.0)
  (Actor|DestroyActor))

(fn ConstructionScript)