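; Magic missile ability that, once activated, automatically fires projectiles at the closest enemy on a looping FireRate timer.
; Each tick searches all BP_EnemyBase actors by distance to the player, then spawns ProjectileCount projectiles just in front of the player toward that target.
; Projectiles receive damage, target and an initial direction fanned across SpreadAngle.
; A separate FireMagicMissile event, not used by the timer, spawns a rotation-based spread with zero damage.
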(event Custom|FireMagicMissile
  (bind _enemy (CallFunction|FindClosestEnemy))
  (Utilities|IsValid _enemy
    (:Is%20Valid
      (for _index (range 0 (- (Variables|Default|GetProjectileCount) 1))
        (Utilities|IsValid _enemy
          (:Is%20Valid
            (bind _returnvalue (Game|SpawnActorfromClass (Variables|Default|GetProjectileClass) (Math|Transform|MakeTransform (+ (Transformation|GetActorLocation (Game|GetPlayerCharacter 0)) (* (Math|Vector|Normalize (Math|Vector|MakeVector (.x (- (Transformation|GetActorLocation _enemy) (Transformation|GetActorLocation (Game|GetPlayerCharacter 0)))) (.y (- (Transformation|GetActorLocation _enemy) (Transformation|GetActorLocation (Game|GetPlayerCharacter 0)))) 0.0)) 1e+02)) (Math|Rotator|CombineRotators (Math|Rotator|MakeRotator (.roll (Math|Rotator|FindLookatRotation (Transformation|GetActorLocation (Game|GetPlayerCharacter 0)) (Transformation|GetActorLocation _enemy))) 0.0 (.yaw (Math|Rotator|FindLookatRotation (Transformation|GetActorLocation (Game|GetPlayerCharacter 0)) (Transformation|GetActorLocation _enemy)))) (Math|Rotator|MakeRotator 0.0 0.0 (- (* _index (Variables|Default|GetSpreadAngle)) (/ (* (- (Variables|Default|GetProjectileCount) 1) (Variables|Default|GetSpreadAngle)) 2.0)))) "1.000000,1.000000,1.000000") "Undefined" "MultiplyWithRoot" 0 0.0 0 "0.000000,0.000000,0.000000" 0))
            (Variables|/Game/Blueprints/Systems/Attack/BP_MagicMissileProjectile.BP_MagicMissileProjectile_C|SetDamage _returnvalue 0.0)))))))

(event Custom|4
  (bind _enemy (CallFunction|FindClosestEnemy))
  (Utilities|IsValid _enemy
    (:Is%20Valid
      (bind _output_get (Variables|Default|SetEnemy _enemy))
      (Variables|Default|SetPlayer%20REF (Game|GetPlayerCharacter 0))
      (for _index (range 0 (- (Variables|Default|GetProjectileCount) 1))
        (Utilities|IsValid _output_get
          (:Is%20Valid
            (bind _finaldirection_ (CallFunction|GetProjectileDirection _index))
            (Game|SpawnActorfromClass (Variables|Default|GetProjectileClass) (Math|Transform|MakeTransform (+ (Transformation|GetActorLocation (Variables|Default|GetPlayer%20REF)) (* (Math|Vector|Normalize (Math|Vector|MakeVector (.x (- (Transformation|GetActorLocation (Variables|Default|GetEnemy)) (Transformation|GetActorLocation (Variables|Default|GetPlayer%20REF)))) (.y (- (Transformation|GetActorLocation (Variables|Default|GetEnemy)) (Transformation|GetActorLocation (Variables|Default|GetPlayer%20REF)))) 0.0)) 1e+02)) "0, 0, 0" "1.000000,1.000000,1.000000") "Undefined" "MultiplyWithRoot" 0 (Variables|Default|GetDamage) (Variables|Default|GetEnemy) _finaldirection_ 0)))))))

(event EventActivateAbility
  (bind _returnvalue (Utilities|Time|SetTimerbyEvent (delegate Custom|4) (Variables|Default|GetFireRate) true))
  (Variables|Default|SetFireTimerHandle _returnvalue))

(fn FindClosestEnemy
  (bind _outactors (Actor|GetAllActorsOfClass "/Game/Blueprints/Systems/Spawner/Enemyies2/BP_EnemyBase.BP_EnemyBase_C"))
  (for _array_element _outactors
    (if (< (Transformation|GetDistanceTo _array_element (Game|GetPlayerCharacter 0)) (LocalVariables|GetShortestDistance))
      (LocalVariables|SetShortestDistance (Transformation|GetDistanceTo _array_element (Game|GetPlayerCharacter 0)))
      (LocalVariables|SetCurrentClosest _array_element)))
  (return (LocalVariables|GetCurrentClosest)))

(fn GetProjectileDirection
  (params (index :type Integer))
  (LocalVariables|SetBaseDirection (Math|Vector|Normalize (- (Transformation|GetActorLocation (Variables|Default|GetEnemy)) (Transformation|GetActorLocation (Variables|Default|GetPlayer%20REF)))))
  (bind _output_get (LocalVariables|SetAngleOffSet (+ (* index (/ (Variables|Default|GetSpreadAngle) (- (Variables|Default|GetProjectileCount) 1))) (/ (* (Variables|Default|GetSpreadAngle) -1.0) 2.0))))
  (return (Math|Vector|RotateVectorAroundAxis (LocalVariables|GetBaseDirection) _output_get "0.000000,0.000000,1.000000")))