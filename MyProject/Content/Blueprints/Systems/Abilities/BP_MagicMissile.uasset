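; Magic Missile ability that, once activated, automatically fires volleys of projectiles from player 0 at the closest enemy on a looping timer.
; Each volley scans all BP_EnemyBase actors for the nearest, then spawns BP_SecondTry projectiles in a centered yaw fan, offset toward the target on the horizontal plane.
; UpgradeAbility steps through weapon levels that add projectiles, shorten the clamped fire interval by restarting the timer, or switch the projectile effect to pierce.
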(event Custom|FireVolley
  (bind _enemy (CallFunction|FindClosestEnemy))
  (Utilities|IsValid _enemy
    (:Is%20Valid
      (for _index (range 0 (- (Variables|Default|GetProjectileCount) 1))
        (Utilities|IsValid _enemy
          (:Is%20Valid
            (Game|SpawnActorfromClass "/Game/Blueprints/Systems/Attack/BP_SecondTry.BP_SecondTry_C" (Math|Transform|MakeTransform (+ (Transformation|GetActorLocation (Game|GetPlayerCharacter 0)) (* (Math|Vector|Normalize (Math|Vector|MakeVector (.x (- (Transformation|GetActorLocation _enemy) (Transformation|GetActorLocation (Game|GetPlayerCharacter 0)))) (.y (- (Transformation|GetActorLocation _enemy) (Transformation|GetActorLocation (Game|GetPlayerCharacter 0)))) 0.0)) 1e+02)) (Math|Rotator|CombineRotators (Math|Rotator|MakeRotator (.roll (Math|Rotator|FindLookatRotation (Transformation|GetActorLocation (Game|GetPlayerCharacter 0)) (Transformation|GetActorLocation _enemy))) 0.0 (.yaw (Math|Rotator|FindLookatRotation (Transformation|GetActorLocation (Game|GetPlayerCharacter 0)) (Transformation|GetActorLocation _enemy)))) (Math|Rotator|MakeRotator 0.0 0.0 (- (* _index (Variables|Default|GetSpreadAngle)) (/ (* (- (Variables|Default|GetProjectileCount) 1) (Variables|Default|GetSpreadAngle)) 2.0)))) "1.000000,1.000000,1.000000") "Undefined" "MultiplyWithRoot" 0 (Variables|Default|GetProjectileEffect) 0)))))))

(event EventActivateAbility
  (bind _returnvalue (Utilities|Time|SetTimerbyEvent (delegate Custom|FireVolley) (Variables|Default|GetFireRate) true))
  (Variables|Default|SetFiringTimer _returnvalue))

(event EventUpgradeAbility
  (bind _result (Math|Integer|IncrementInt (Variables|Default|Getweaponlvl))
    (:%20%20
      (switch int _result
        (:1
          (Math|Integer|IncrementInt (Variables|Default|GetProjectileCount) :!label _label
            (:%20%20
              (Development|PrintString "Multi shot"))))
        (:2
          (bind _output_get (Variables|Default|SetFireRate (Math|Float|Clamp(Float) (* (Variables|Default|GetFireRate) 0.9) 0.2) :!label _label_2))
          (Utilities|Time|ClearandInvalidateTimerbyHandle (Variables|Default|GetFiringTimer))
          (bind _returnvalue (Utilities|Time|SetTimerbyEvent (delegate Custom|FireVolley) (Variables|Default|GetFireRate) true))
          (Variables|Default|SetFiringTimer _returnvalue)
          (Development|PrintString (Utilities|String|ToString(Float) _output_get)))
        (:3
          (goto _label))
        (:4
          (Development|PrintString "Pierce!!!!")
          (Variables|Default|SetProjectileEffect "NewEnumerator1"))
        (:5
          (goto _label_2))
        (:6
          (goto _label))
        (:7
          (goto _label_2))
        (:8
          (goto _label_2))))))

(fn FindClosestEnemy
  (bind _outactors (Actor|GetAllActorsOfClass "/Game/Blueprints/Systems/Spawner/Enemyies2/BP_EnemyBase.BP_EnemyBase_C"))
  (for _array_element _outactors
    (if (< (Transformation|GetDistanceTo _array_element (Game|GetPlayerCharacter 0)) (LocalVariables|GetShortestDistance))
      (LocalVariables|SetShortestDistance (Transformation|GetDistanceTo _array_element (Game|GetPlayerCharacter 0)))
      (LocalVariables|SetCurrentClosest _array_element)))
  (return (LocalVariables|GetCurrentClosest)))