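; BP_RewardGenerator picks a requested number of random rewards from an assigned Data Table.
; GetRandomRewards copies the RewardTable rows into a temporary pool, then makes weighted picks by subtracting each row's Weight from a random roll within the total.
; When AllowDuplicates is off, each pick leaves the pool and the total weight is recalculated for the next roll.
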(event EventBeginPlay)

(event EventTick
  (params (DeltaSeconds :type Float%20%28single-precision%29)))

(fn GetRandomRewards
  (params (Amount%20to%20Generate :type Integer))
  ;[1 0.7568 0.9322] Add a Data Table to component before using
  (bind _outrownames (DataTable|GetDataTableRowNames (Variables|Default|GetRewardTable)))
  (for _array_element _outrownames
    (bind _returnvalue (Utilities|GetDataTableRow (Variables|Default|GetRewardTable) _array_element)
      (:then
        (Utilities|Array|Add (LocalVariables|GetTempPool) _returnvalue))))
  (for _index (range 1 Amount%20to%20Generate)
    ;[1 0.1305 0.07081] Total weight for each item in loop
    (LocalVariables|SetTotalWeight 0.0)
    (for _array_element_2 (LocalVariables|GetTempPool)
      (LocalVariables|SetTotalWeight (+ (LocalVariables|GetTotalWeight) (.Weight (Utilities|Struct|BreakS_RewardData _array_element_2)))))
    ;[1 0.8955 0.2435] Get random value, itterate  trough Current Possible rewards, if duplicates are not allowed remove item
    (LocalVariables|SetRandomValue (Math|Random|RandomFloatinRange 0.0 (LocalVariables|GetTotalWeight)))
    (bind _array_element_3 (Utilities|Array|ForEachLoopwithBreak (LocalVariables|GetTempPool) :!label _label)
      (:LoopBody
        (if (<= (LocalVariables|GetRandomValue) (.Weight (Utilities|Struct|BreakS_RewardData _array_element_3)))
          (Utilities|Array|Add (LocalVariables|GetSelected%20Rewards%20local) _array_element_3)
          (if (not (Variables|Default|GetbAllowDuplicates))
            (Utilities|Array|RemoveItem (LocalVariables|GetTempPool) _array_element_3)
            (goto _label Break)
            (else
              (goto _label Break)))
          (else
            (LocalVariables|SetRandomValue (- (LocalVariables|GetRandomValue) (.Weight (Utilities|Struct|BreakS_RewardData _array_element_3)))))))))
  ;[0.1165 1 0.2316] Your Rewards
  (return (LocalVariables|GetSelected%20Rewards%20local)))