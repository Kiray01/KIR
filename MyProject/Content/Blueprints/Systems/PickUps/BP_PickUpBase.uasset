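; BP_PickUpBase is a base pickup actor that randomly becomes a small, mid or large mana pickup at BeginPlay.
; Nested random rolls weight the type so that large is rarest and small is most common.
; When a BP_CharacterBase overlaps its sphere, it passes the type to that character's OnPickUp and destroys itself.
; SetPickUp is an unfinished switch on the type and is never run.
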(event OnComponentBeginOverlap(Sphere)
  (params (OverlappedComponent :type Primitive%20Component%20Object%20Reference) (OtherActor :type Actor%20Object%20Reference) (OtherComp :type Primitive%20Component%20Object%20Reference) (OtherBodyIndex :type Integer) (bFromSweep :type Boolean) (SweepResult :type Hit%20Result%20Structure%20%28by%20ref%29))
  (bind _asbp_character_base (Utilities|Casting|CastToBP_CharacterBase OtherActor))
  (Default|OnPickUp _asbp_character_base (Variables|Default|GetPickUpType))
  (Actor|DestroyActor))

(event EventBeginPlay
  (bind _returnvalue (Math|Random|RandomFloatinRange 0.0 1.0))
  (if (<= _returnvalue 0.1)
    (Variables|Default|SetPickUpType "NewEnumerator2")
    (elif (<= _returnvalue 0.35)
      (Variables|Default|SetPickUpType "NewEnumerator1")
      (else
        (Variables|Default|SetPickUpType "NewEnumerator0")))))

(fn ConstructionScript)

(fn SetPickUp
  (switch Utilities|FlowControl|Switch|SwitchonE_PickUpTypes (Variables|Default|GetPickUpType)))