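; Map manager that creates an endless world around the player by recycling a fixed 5x5 grid of BP_MapTile actors.
; A looping timer tracks the player's grid cell and, when it changes, wraps distant tiles to the opposite side instead of spawning new ones.
; A slower timer moves the referenced navigation volume to the player when they stray too far from it.
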(event Custom|Teleport%20Navigation%20Lolume
  (bind _returnvalue (Game|GetPlayerCharacter 0))
  (bind _returnvalue_2 (Transformation|GetActorLocation _returnvalue))
  (if (not (Utilities|Operators|EqualEqual _returnvalue_2 (Transformation|GetActorLocation (Variables|Default|GetNavREF)) 5e+03))
    (Transformation|SetActorLocation (Variables|Default|GetNavREF) _returnvalue_2 false false)))

(event EventBeginPlay
  (Utilities|FlowControl|Sequence
    (:then_0
      ;[1 0.3582 0.9385] Spawn  Tiles
      (for _index (range -2 2)
        (for _index_2 (range -2 2)
          (bind _returnvalue (Game|SpawnActorfromClass "/Game/Blueprints/Systems/Map/BP_MapTile.BP_MapTile_C" (Math|Transform|MakeTransform (Math|Vector|MakeVector (* (Variables|Default|GetTilesize) _index) (* (Variables|Default|GetTilesize) _index_2) 0.0) "0, 0, 0" "1.000000,1.000000,1.000000") "Undefined" "MultiplyWithRoot" 0 0))
          (Utilities|Array|Add (Variables|Default|GetMapTiles) _returnvalue)))
      (Utilities|Time|SetTimerbyFunctionName 0 "CheckPlayerGridPos" 2.5 true))
    (:then_1
      (Utilities|Time|SetTimerbyEvent (delegate Custom|Teleport%20Navigation%20Lolume) 4e+01 true))))

(fn ConstructionScript)

(fn RepositionTiles
  (bind _returnvalue (Game|Player|GetPlayerPawn 0))
  (bind _returnvalue_2 (Transformation|GetActorLocation _returnvalue))
  (for _array_element (Variables|Default|GetMapTiles)
    (LocalVariables|SetDx (- (.x _returnvalue_2) (.x (Transformation|GetActorLocation _array_element))))
    (LocalVariables|SetDy (- (.y _returnvalue_2) (.y (Transformation|GetActorLocation _array_element))))
    (Utilities|FlowControl|Sequence
      (:then_0
        (Utilities|FlowControl|Sequence
          (:then_0
            (if (> (LocalVariables|GetDx) (* (Variables|Default|GetTilesize) 2.5))
              (Transformation|AddActorWorldOffset _array_element (Math|Vector|MakeVector (* (Variables|Default|GetTilesize) 5.0) 0.0 0.0))))
          (:then_1
            (if (< (LocalVariables|GetDx) (* (Variables|Default|GetTilesize) -2.5))
              (Transformation|AddActorWorldOffset _array_element (Math|Vector|MakeVector (* (Variables|Default|GetTilesize) -5.0) 0.0 0.0))))))
      (:then_1
        (Utilities|FlowControl|Sequence
          (:then_0
            (if (> (LocalVariables|GetDy) (* (Variables|Default|GetTilesize) 2.5))
              (Transformation|AddActorWorldOffset _array_element (Math|Vector|MakeVector 0.0 (* (Variables|Default|GetTilesize) 5.0) 0.0))))
          (:then_1
            (if (< (LocalVariables|GetDy) (* (Variables|Default|GetTilesize) -2.5))
              (Transformation|AddActorWorldOffset _array_element (Math|Vector|MakeVector 0.0 (* (Variables|Default|GetTilesize) -5.0) 0.0)))))))))

(fn CheckPlayerGridPos
  (bind _returnvalue (Game|Player|GetPlayerPawn 0))
  (bind _returnvalue_2 (Transformation|GetActorLocation _returnvalue))
  (Variables|Default|SetX_Grid (Math|Float|Round (/ (.x _returnvalue_2) (Variables|Default|GetTilesize))))
  (Variables|Default|SetY_Grid (Math|Float|Round (/ (.y _returnvalue_2) (Variables|Default|GetTilesize))))
  (if (or (!= (Variables|Default|GetX_Grid) (.x (Variables|Default|GetLastPlayerGridPos))) (!= (Variables|Default|GetY_Grid) (.y (Variables|Default|GetLastPlayerGridPos))))
    (Variables|Default|SetLastPlayerGridPos (Math|Vector2D|MakeVector2D (Math|Conversions|ToFloat(Integer) (Variables|Default|GetX_Grid)) (Math|Conversions|ToFloat(Integer) (Variables|Default|GetY_Grid))))
    (CallFunction|RepositionTiles)))