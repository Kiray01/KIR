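; BP_EnemyBase is the base enemy that chases the player, deals contact damage and grants experience when killed.
; On spawn it scales max health by a difficulty multiplier and starts a looping timer that re-issues AIMoveTo toward the player character.
; Capsule overlap with a BP_CharacterBase applies fixed damage.
; Incoming hits reduce health, and at zero it destroys itself and adds its base EXP to the player.
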(event OnComponentBeginOverlap(CapsuleComponent)
  (params (OverlappedComponent :type Primitive%20Component%20Object%20Reference) (OtherActor :type Actor%20Object%20Reference) (OtherComp :type Primitive%20Component%20Object%20Reference) (OtherBodyIndex :type Integer) (bFromSweep :type Boolean) (SweepResult :type Hit%20Result%20Structure%20%28by%20ref%29))
  (bind _asbp_character_base (Utilities|Casting|CastToBP_CharacterBase OtherActor))
  (Default|TakeDamage _asbp_character_base (Utilities|Struct|MakeS_HitInfo 2e+01 self "0.000000,0.000000,0.000000" "0.000000,0.000000,0.000000" false)))

(event Custom|UpdateMovement
  (AI|AIMoveTo self "0, 0, 0" (Variables|Default|GetPlayerRef) 5e+01 false))

(event EventBeginPlay
  (Variables|Default|SetPlayerRef (Game|GetPlayerCharacter 0))
  (Utilities|Time|SetTimerbyEvent (delegate Custom|UpdateMovement) 0.2 true)
  (Variables|Default|SetMaxHealth (* (Variables|Default|GetMaxHealth) (Variables|Default|GetDifficultyMultiplayer)))
  (Variables|Default|SetCurrentHealth (Variables|Default|GetMaxHealth)))

(event EventTakeDamage
  (params (HitData :type S%20Hit%20Info%20Structure))
  (bind _output_get (Variables|Default|SetCurrentHealth (- (Variables|Default|GetCurrentHealth) (.damageamount HitData))))
  (if (<= _output_get 0.0)
    (Actor|DestroyActor)
    (bind _asbp_character_base (Utilities|Casting|CastToBP_CharacterBase (Variables|Default|GetPlayerRef)))
    (Default|AddEXP _asbp_character_base (Variables|Default|GetBaseEXP))))

(fn ConstructionScript)