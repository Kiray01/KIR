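; Spawn director that periodically spawns waves of enemies around the player, scaling with game time.
; Each looping timer tick sets a credit budget from SpawnCurve and spends it over capped attempts.
; GetEnemyToSpawn filters EnemyTable by cost and minimum time, then makes a weighted random pick.
; Spawns use random navmesh-projected points within a distance range, face the player and receive a ScaleCurve difficulty multiplier.
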(event Custom|SpawnWave
  (bind _returnvalue (Utilities|Time|GetGameTimeinSeconds))
  (bind _returnvalue_2 (Math|Random|RandomFloatinRange 0.0 3.6e+02))
  (bind _returnvalue_3 (Game|GetPlayerCharacter 0))
  (bind _minspawndistance (Variables|Default|GetMinSpawnDistance))
  (bind _maxspawndistance (Variables|Default|GetMaxSpawnDistance))
  (bind _returnvalue_4 (Math|Random|RandomFloatinRange _minspawndistance _maxspawndistance))
  (bind _returnvalue_5 (Math|Rotator|MakeRotator 0.0 0.0 _returnvalue_2))
  (bind _returnvalue_6 (Transformation|GetActorLocation _returnvalue_3))
  (bind _returnvalue_7 (Math|Vector|GetForwardVector _returnvalue_5))
  (bind _returnvalue_8 (* _returnvalue_7 _returnvalue_4))
  (bind _returnvalue_9 (+ _returnvalue_8 _returnvalue_6))
  (bind (_projectedlocation _returnvalue_10) (AI|Navigation|ProjectPointtoNavigation _returnvalue_9 0 0 "500.000000,500.000000,2000.000000"))
  ;[1 0.3546 0.2648] Assign credits
  (Variables|Default|SetCurrentCredits (Math|Float|Truncate (Math|Curves|GetFloatValue (Variables|Default|GetSpawnCurve) _returnvalue)))
  (Utilities|FlowControl|ForLoopwithBreak 0 (- (Variables|Default|GetMaxAttempts) 1) :!label _label
    (:LoopBody
      (bind (_seletedenemy _cost _success) (CallFunction|GetEnemytoSpawn (Variables|Default|GetCurrentCredits) _returnvalue))
      (if _success
        ;[1 0.6317 0.9079] Reduce Credits after each iteration
        (Variables|Default|SetCurrentCredits (- (Variables|Default|GetCurrentCredits) _cost))
        (if _returnvalue_10
          (Game|SpawnActorfromClass _seletedenemy (Math|Transform|MakeTransform _projectedlocation (Math|Rotator|FindLookatRotation _projectedlocation _returnvalue_6) "1.000000,1.000000,1.000000") "Undefined" "MultiplyWithRoot" 0 (Math|Curves|GetFloatValue (Variables|Default|GetScaleCurve) _returnvalue) 0))
        (else
          (goto _label Break))))))

(event EventBeginPlay
  (Utilities|Time|SetTimerbyEvent (delegate Custom|SpawnWave) 2.0 true))

(fn ConstructionScript)

(fn GetEnemytoSpawn
  (params (CurrentCredits :type Integer) (GameTime :type Float%20%28double-precision%29))
  ;[0.2624 0.1136 1] Set up Candidates
  (Utilities|Array|Clear (LocalVariables|GetCurrentCandidates))
  (bind _outrownames (DataTable|GetDataTableRowNames (Variables|Default|GetEnemyTable)))
  (for _array_element _outrownames
    (bind _returnvalue (Utilities|GetDataTableRow (Variables|Default|GetEnemyTable) _array_element)
      (:then
        (if (and (>= (Variables|Default|GetCurrentCredits) (.CreditCost (Utilities|Struct|BreakS_EnemyData _returnvalue))) (>= GameTime (.MinTime (Utilities|Struct|BreakS_EnemyData _returnvalue))))
          (Utilities|Array|Add (LocalVariables|GetCurrentCandidates) _returnvalue)))))
  ;[1 0.4154 0.2243] NOT 0?
  (if (== (Utilities|Array|Length (LocalVariables|GetCurrentCandidates)) 0)
    (return 0 0 false)
    (else
      ;[0.3767 0.9001 1] Total Weight
      (LocalVariables|SetTotalWeight 0.0)
      (for _array_element_2 (LocalVariables|GetCurrentCandidates)
        (LocalVariables|SetTotalWeight (+ (LocalVariables|GetTotalWeight) (.SpawnChance (Utilities|Struct|BreakS_EnemyData _array_element_2)))))
      ;[1 0.3441 0.4541] Iterate till Enemy type is found
      (LocalVariables|SetRandomValue (Math|Random|RandomFloatinRange 0.0 (LocalVariables|GetTotalWeight)))
      (bind _array_element_3 (Utilities|Array|ForEachLoopwithBreak (LocalVariables|GetCurrentCandidates))
        (:LoopBody
          (if (<= (LocalVariables|GetRandomValue) (.SpawnChance (Utilities|Struct|BreakS_EnemyData _array_element_3)))
            (return (.ActorClass (Utilities|Struct|BreakS_EnemyData _array_element_3)) (.CreditCost (Utilities|Struct|BreakS_EnemyData _array_element_3)) true)
            (else
              (LocalVariables|SetRandomValue (- (LocalVariables|GetRandomValue) (.SpawnChance (Utilities|Struct|BreakS_EnemyData _array_element_3)))))))))))