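; Spawn director that spawns enemies around the player on a credit budget that varies with game time.
; A fast looping timer runs SpawnWave, which resets the budget from a curve and buys enemies until none qualify or attempts run out.
; GetEnemyToSpawn filters data table rows by cost and minimum time, then makes a weighted random pick.
; Enemies spawn at random navmesh-projected points within a distance range, facing the player, with debug prints.
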(event Custom|SpawnWave
  (bind _returnvalue (Utilities|Time|GetGameTimeinSeconds))
  (bind _returnvalue_2 (Math|Random|RandomUnitVector))
  (bind _returnvalue_3 (Game|GetPlayerCharacter 0))
  (bind _minspawndistance (Variables|Default|GetMinSpawnDistance))
  (bind _maxspawndistance (Variables|Default|GetMaxSpawnDistance))
  (bind _returnvalue_4 (Math|Random|RandomFloatinRange _minspawndistance _maxspawndistance))
  (bind _returnvalue_5 (Transformation|GetActorLocation _returnvalue_3))
  (bind _returnvalue_6 (* _returnvalue_2 _returnvalue_4))
  (bind _returnvalue_7 (+ _returnvalue_6 _returnvalue_5))
  (bind (_projectedlocation _returnvalue_8) (AI|Navigation|ProjectPointtoNavigation _returnvalue_7 0 0 "500.000000,500.000000,1000.000000"))
  (Variables|Default|SetSpawned 0)
  (bind _output_get (Variables|Default|SetCurrentCredits (Math|Float|Truncate (Math|Curves|GetFloatValue (Variables|Default|GetSpawnCurve) _returnvalue))))
  (Development|PrintString (Utilities|String|Append (Utilities|String|Append "Time: " (Utilities|String|ToString(Float) _returnvalue)) (Utilities|String|Append " Budget: " (Utilities|String|ToString(Integer) _output_get))) true true "(R=1.000000,G=0.000000,B=0.689769,A=1.000000)" 2.0 "Budget")
  (Utilities|FlowControl|ForLoopwithBreak 0 (- (Variables|Default|GetMaxAttempts) 1) :!label _label
    (:LoopBody
      (bind (_seletedenemy _cost _success) (CallFunction|GetEnemytoSpawn (Variables|Default|GetCurrentCredits) _returnvalue))
      ;[1 1 1] Fix spaw rate
      (if _success
        (Variables|Default|SetCurrentCredits (- (Variables|Default|GetCurrentCredits) _cost))
        (if _returnvalue_8
          (Game|SpawnActorfromClass _seletedenemy (Math|Transform|MakeTransform _projectedlocation (Math|Rotator|FindLookatRotation _projectedlocation _returnvalue_5) "1.000000,1.000000,1.000000") "Undefined" "MultiplyWithRoot" 0 0)
          (Math|Integer|IncrementInt (Variables|Default|GetSpawned)
            (:%20%20
              (Development|PrintString (Utilities|String|Append (Utilities|String|Append "Bought:  " (Utilities|GetClassDisplayName _seletedenemy)) (Utilities|String|Append " Cost: " (Utilities|String|ToString(Integer) _cost))) true true "(R=0.195485,G=1.000000,B=0.347344,A=1.000000)" 2.0 ""))))
        (else
          (goto _label Break))))
    (:Completed
      (Development|PrintString (Utilities|String|ToString(Integer) (Variables|Default|GetSpawned)))
      (Utilities|FlowControl|Delay 5.0))))

(event EventBeginPlay
  (Utilities|Time|SetTimerbyEvent (delegate Custom|SpawnWave) 0.1 true))

(fn ConstructionScript)

(fn GetEnemytoSpawn
  (params (CurrentCredits :type Integer) (GameTime :type Float%20%28double-precision%29))
  ;[0.2624 0.1136 1] Set up Candidates
  (Utilities|Array|Clear (LocalVariables|GetCurrentCandidates))
  (bind _outrownames (DataTable|GetDataTableRowNames (Variables|Default|GetEnemyTable)))
  (for _array_element _outrownames
    (bind _returnvalue (Utilities|GetDataTableRow (Variables|Default|GetEnemyTable) _array_element)
      (:then
        (if (and (>= (Variables|Default|GetCurrentCredits) (.CreditCost (Utilities|Struct|BreakS_EnemyData _returnvalue))) (>= GameTime (.MinTime (Utilities|Struct|BreakS_EnemyData _returnvalue))))
          (Utilities|Array|Add (LocalVariables|GetCurrentCandidates) _returnvalue)))))
  ;[1 0.4154 0.2243] NOT 0?
  (if (== (Utilities|Array|Length (LocalVariables|GetCurrentCandidates)) 0)
    (return 0 0 false)
    (else
      ;[0.3767 0.9001 1] Total Weight
      (LocalVariables|SetTotalWeight 0.0)
      (for _array_element_2 (LocalVariables|GetCurrentCandidates)
        (LocalVariables|SetTotalWeight (+ (LocalVariables|GetTotalWeight) (.SpawnChance (Utilities|Struct|BreakS_EnemyData _array_element_2)))))
      ;[1 0.3441 0.4541] Works
      (LocalVariables|SetRandomValue (Math|Random|RandomFloatinRange 0.0 (LocalVariables|GetTotalWeight)))
      (bind _array_element_3 (Utilities|Array|ForEachLoopwithBreak (LocalVariables|GetCurrentCandidates))
        (:LoopBody
          (if (<= (LocalVariables|GetRandomValue) (.SpawnChance (Utilities|Struct|BreakS_EnemyData _array_element_3)))
            (return (.ActorClass (Utilities|Struct|BreakS_EnemyData _array_element_3)) (.CreditCost (Utilities|Struct|BreakS_EnemyData _array_element_3)) true)
            (else
              (LocalVariables|SetRandomValue (- (LocalVariables|GetRandomValue) (.SpawnChance (Utilities|Struct|BreakS_EnemyData _array_element_3)))))))))))